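; Interactive door actor that the player opens and closes with the Do input action while overlapping it.
; Begin and end overlap enable and disable input for player controller 0, without checking which actor overlaps.
; The DoorRotation timeline drives the door's relative yaw, playing to open and reversing to close.
; Tick derives IsClosed each frame from whether the timeline's rotation value is below one degree.
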(event Collision|EventActorBeginOverlap
  (params (OtherActor :type Actor%20Object%20Reference))
  (Input|EnableInput (Game|GetPlayerController 0)))

(event Collision|EventActorEndOverlap
  (params (OtherActor :type Actor%20Object%20Reference))
  (Input|DisableInput (Game|GetPlayerController 0)))

(event EventTick
  (params (DeltaSeconds :type Float%20%28single-precision%29))
  (Variables|Default|SetIsClosed (< (stale Input|ActionEvents|InputActionDo _door_rot) 1.0)))

(event Input|ActionEvents|InputActionDo
  (params (Key :type Key%20Structure :default "AnyKey"))
  (:Pressed
    (if (Variables|Default|GetIsClosed)
      (bind _door_rot (Timeline|DoorRotation Play)
        (:Update
          (Transformation|SetRelativeRotation (Variables|Default|GetDoor) (Math|Rotator|MakeRotator 0.0 0.0 _door_rot) false false)))
      (else
        (Timeline|DoorRotation Reverse)))))

(fn ConstructionScript)

(fn NewFunction0)